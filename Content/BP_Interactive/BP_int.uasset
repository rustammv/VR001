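; Interactive prop Actor that can be highlighted and picked up by BP_MotionController, gated by HighLightable and PickUpable flags.
; The construction script applies the chosen mesh, rebuilds an editable per-slot material list when it changes, and applies those materials.
; Highlighting uses custom depth stencil, with a retriggerable delay clearing it unless refreshed.
; Pickup attaches it to the controller; dropping detaches it and optionally simulates physics for one second.
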(event `self.ReceiveBeginPlay`)

(event `self.ReceiveTick`
  (params (DeltaSeconds :type "Float (single-precision)")))

(event `/Game/Interface/I_HighLightable.OnHighLight`
  (params (DepthStencil :type Integer))
  (if (`self.HighLightable`)
    (`/Game/BP_Interactive/BP_FurnetureParts/FL_HighLightable.StartHighLight` (`self.SMArray`) DepthStencil)
    (set `self.Timer` 0.1)
    (`KismetSystemLibrary.RetriggerableDelay` (`self.Timer`))
    (`/Game/BP_Interactive/BP_FurnetureParts/FL_HighLightable.EndHighLight` (`self.SMArray`))))

(event `/Game/Interface/I_Pickupble.Pickup`
  (params (AttachTo :type "SceneComponent Object Reference"))
  (if (`self.PickUpable`)
    (set `self.MotionController` AttachTo)
    (set `self.isPicking` true)
    (`PrimitiveComponent.SetSimulatePhysics` (`self.StaticMeshComponent`) false)
    (`SceneComponent.K2_AttachToComponent` (`self.K2_GetRootComponent`) (`self.MotionController`) "None" "KeepWorld" "KeepWorld" "KeepWorld" false)))

(event `/Game/Interface/I_Pickupble.Drop`
  (if (`self.PickUpable`)
    (set `self.isPicking` false)
    (`PrimitiveComponent.SetSimulatePhysics` (`self.StaticMeshComponent`) (`self.UsePhysics`))
    (`self.K2_DetachFromActor` "KeepWorld" "KeepWorld" "KeepWorld")
    (`KismetSystemLibrary.Delay` 1.0)
    (`PrimitiveComponent.SetSimulatePhysics` (`self.StaticMeshComponent`) false)))

(fn `ApplyMaterials`
  (for (_array_element _array_index) (`self.Mat`)
    (`PrimitiveComponent.SetMaterial` (`self.StaticMeshComponent`) _array_index (break `/Game/Struct/Struct_SMMat` _array_element)))
  (return))

(fn `BeginFocus`
  (for _array_element (`self.SMArray`)
    (`PrimitiveComponent.SetRenderCustomDepth` _array_element true)))

(fn `EndFocus`
  (for _array_element (`self.SMArray`)
    (`PrimitiveComponent.SetRenderCustomDepth` _array_element false)))

(fn `UserConstructionScript`
  (locals (IsNewSM :type Boolean) (Index :type Integer))
  (bind _smarray (`self.SMArray`))
  (bind _staticmeshcomponent (`self.StaticMeshComponent`))
  (`KismetArrayLibrary.Array_Clear` _smarray)
  (`KismetArrayLibrary.Array_Add` _smarray (`self.StaticMeshComponent`))
  (for _array_element (`self.SMArray`)
    (`PrimitiveComponent.SetRenderCustomDepth` _array_element false)
    (`PrimitiveComponent.SetCustomDepthStencilValue` _array_element (`self.DepthStencilValue`))
    (`PrimitiveComponent.SetSimulatePhysics` _array_element false))
  (bind _output_get (set `local.IsNewSM` (!= (`StaticMeshComponent.StaticMesh` (`self.StaticMeshComponent`)) (`self.SM`))))
  (if _output_get
    (`StaticMeshComponent.SetStaticMesh` _staticmeshcomponent (`self.SM`))
    (set `self.CountMaterial` (- (`PrimitiveComponent.GetNumMaterials` _staticmeshcomponent) 1))
    ;[1 1 1] Очищаем масив с материалами, добавляем все материалы из SM и создаём нужное количестао ечеек и заполняем их
    (`KismetArrayLibrary.Array_Clear` (`self.Mat`))
    (for _index (range (+ (`self.CountMaterial`) 1))
      (set `local.Index` _index)
      (`KismetArrayLibrary.Array_Add` (`self.Mat`))
      (`KismetArrayLibrary.Array_Set` (`self.Mat`) (`local.Index`) (make `/Game/Struct/Struct_SMMat` (`StaticMesh.GetMaterial` (`self.SM`) (`local.Index`)) (`|GetArrayItem` (`MeshComponent.GetMaterialSlotNames` (`self.StaticMeshComponent`)) (`local.Index`)))))
    (`self.ApplyMaterials`)
    (else
      (`self.ApplyMaterials`))))