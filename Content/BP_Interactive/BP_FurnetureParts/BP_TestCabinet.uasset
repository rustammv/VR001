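; BP_TestCabinet is a test cabinet Blueprint assembled from BP_Openable child actors, with facade materials that can be changed per group.
; The construction script rebuilds the cabinet's GroupMaterial collection from the main material of each openable child.
; SetMaterialGroup walks all child actors and applies the given facade material to openables whose own GroupMaterial matches the requested group index.
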(event `SetMaterialGroup`
  (params (GroupIndex :type Integer) (Material :type "MaterialInterface Object Reference"))
  (for _array_element (`self.GetAllChildActors` true)
    (bind _asbp_openable (cast `/Game/BP_Interactive/BP_FurnetureParts/BP_Openable` _array_element))
    (if (== (`/Game/BP_Interactive/BP_FurnetureParts/BP_Openable.GroupMaterial` _asbp_openable) GroupIndex)
      (`/Game/BP_Interactive/BP_FurnetureParts/BP_Openable.SetMaterialFasade` _asbp_openable Material))))

(fn `UserConstructionScript`
  (locals (NewLocalVar_0 :type "Array of Actor Object Reference"))
  (`KismetArrayLibrary.Array_Clear` (`self.GroupMaterial`))
  (for _array_element (`self.GetAllChildActors` true)
    (bind _asbp_openable (cast `/Game/BP_Interactive/BP_FurnetureParts/BP_Openable` _array_element))
    (`KismetArrayLibrary.Array_Add` (`self.GroupMaterial`) (`/Game/BP_Interactive/BP_FurnetureParts/BP_Openable.GetMaterialMain` _asbp_openable))))