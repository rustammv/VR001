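; BP_StaticGen is an interactive furniture part built on a procedural mesh that can be highlighted through custom depth.
; The construction script makes that mesh the only entry in SMArray, turns custom depth off, assigns the stencil value and disables physics simulation.
; GetMaterialMain returns the material of the mesh's last section as the main material, and the event graph holds no logic.
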(event `self.ReceiveBeginPlay`)

(event `self.ReceiveTick`
  (params (DeltaSeconds :type "Float (single-precision)")))

(fn `GetMaterialMain`
  (returns (MaterialMain :type "MaterialInterface Object Reference"))
  (bind _proceduralmesh (`self.ProceduralMesh`))
  (return (`PrimitiveComponent.GetMaterial` _proceduralmesh (- (`ProceduralMeshComponent.GetNumSections` _proceduralmesh) 1))))

(fn `UserConstructionScript`
  (bind _smarray (`self.SMArray`))
  ;[0.2031 0.2031 0.2031] Очищаем и добавляем меши которые будут подсвечиватся
  (`KismetArrayLibrary.Array_Clear` _smarray)
  (`KismetArrayLibrary.Array_Add` _smarray (`self.ProceduralMesh`))
  (for _array_element (`self.SMArray`)
    (`PrimitiveComponent.SetRenderCustomDepth` _array_element false)
    (`PrimitiveComponent.SetCustomDepthStencilValue` _array_element (`self.DepthStencilValue`))
    (`PrimitiveComponent.SetSimulatePhysics` _array_element false)))