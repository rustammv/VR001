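; Interactive hinged door that opens and closes on a Timeline-driven rotation of its pivot, only while the Target trigger is overlapped.
; Construction script assigns configurable meshes and calls SetupDoor, which places trims by wall thickness and pivot, knob, hinges and trigger by door width and side.
; Side-switch events rerun SetupDoor to flip the swing.
; Focus events briefly toggle focus, apparently for a custom-depth outline.
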(event `self.OnFocus`
  ;[1 1 1] OnFocus PP_Outline knob
  (if (`self.IsNearTrigger`)
    (`self.BeginFocus`)
    (set `self.Timer_0` 0.1)
    (`KismetSystemLibrary.RetriggerableDelay` (`self.Timer_0`))
    (`KismetSystemLibrary.Delay` 0.2)
    (`self.EndFocus`)))

(event `DoorSideTurn_1`
  (set `self.SideOpen` (not (`self.SideOpen`)))
  (`self.SetupDoor` :!label _label))

(event `self.Target.OnComponentBeginOverlap`
  (params (OverlappedComponent :type "PrimitiveComponent Object Reference") (OtherActor :type "Actor Object Reference") (OtherComp :type "PrimitiveComponent Object Reference") (OtherBodyIndex :type Integer) (bFromSweep :type Boolean) (SweepResult :type "HitResult Structure (by ref)"))
  (set `self.IsNearTrigger` true))

(event `DoorSideLeft_1`
  (set `self.SideOpen` false)
  (goto _label))

(event `self.Target.OnComponentEndOverlap`
  (params (OverlappedComponent :type "PrimitiveComponent Object Reference") (OtherActor :type "Actor Object Reference") (OtherComp :type "PrimitiveComponent Object Reference") (OtherBodyIndex :type Integer))
  (set `self.IsNearTrigger` false))

(event `DoorSideRight_1`
  (set `self.SideOpen` true)
  (goto _label))

(event `self.DoorOpenClose`
  (`KismetSystemLibrary.PrintString` "doorOpen")
  (if (`self.IsNearTrigger`)
    (if (`self.DoorIsRotate`)
      _
      (elif (`self.DoorOpenStatus`)
        (set `self.DoorOpenStatus` false)
        (set `self.DoorIsRotate` true)
        (bind (_direction _driver) (`Timeline|Timeline_0` :!via `Reverse` :!label _label_2)
          (:`Update`
            (`SceneComponent.K2_SetRelativeRotation` (`self.Scene`) (`KismetMathLibrary.RLerp` (`self.StartDoor`) (`self.EndDoor`) _driver) false true))
          (:`Finished`
            (set `self.DoorIsRotate` false)))
        (else
          (set `self.DoorOpenStatus` true)
          (set `self.DoorIsRotate` true)
          (goto _label_2))))))

(event `self.ReceiveBeginPlay`
  (`PrimitiveComponent.SetCollisionEnabled` (`self.SM_Door`) "QueryAndPhysics")
  (`PrimitiveComponent.SetCollisionEnabled` (`self.SM_Frame`) "QueryAndPhysics"))

(fn `OnRep_StartDoor`)

(fn `SetupDoor`
  (bind _wallthickness (`self.WallThickness`))
  (bind _returnvalue (- (`self.Width`) 0.0))
  (bind _returnvalue_2 (- (`self.Width`) 0.0))
  (bind _returnvalue_3 (- (`self.Width`) 5.0))
  ;[1 1 1] If Door opened then rotate scene to closed, else nothing
  (if (`self.DoorOpenStatus`)
    (`SceneComponent.K2_SetRelativeRotation` (`self.Scene`) (`self.StartDoor`) false true))
  ;[1 1 1] Trim Position
  (if (<= (`self.WallThickness`) 16.700001)
    (set `self.OffSetThimOutSide` (* _wallthickness -1.0))
    (set `self.OffSetThimInside` 0.0)
    (else
      (set `self.OffSetThimOutSide` -16.700001)
      (set `self.OffSetThimInside` (- _wallthickness 16.700001))))
  (`SceneComponent.K2_SetRelativeLocation` (`self.SM_TrimInSide`) (`KismetMathLibrary.MakeVector` (`self.OffSetThimInside`)) false true)
  (`SceneComponent.K2_SetRelativeLocation` (`self.SM_TrimOutSide`) (`KismetMathLibrary.MakeVector` (`self.OffSetThimOutSide`)) false true)
  ;[1 1 1] Scene Position
  (if (`self.SideOpen`)
    (set `self.OffsetScene` _returnvalue)
    (else
      (set `self.OffsetScene` (* _returnvalue -1.0))))
  (`SceneComponent.K2_SetRelativeLocation` (`self.Scene`) (`KismetMathLibrary.MakeVector` -0.5 (`self.OffsetScene`)) false false)
  ;[1 1 1] Door Position
  (if (`self.SideOpen`)
    (set `self.OffsetDoor` (* _returnvalue_2 -1.0))
    (set `self.EndDoor` (struct :`Yaw` 90.0))
    (else
      (set `self.OffsetDoor` _returnvalue_2)
      (set `self.EndDoor` (struct :`Yaw` -90.0))))
  (`SceneComponent.K2_SetRelativeLocation` (`self.SM_Door`) (`KismetMathLibrary.MakeVector` -2.0 (`self.OffsetDoor`)) false true)
  ;[1 1 1] Knob and Hinges Position Rotation
  (if (`self.SideOpen`)
    (set `self.KnobRotate` (struct :`Yaw` -180.0))
    (set `self.OffsetKnob` (* _returnvalue_3 -1.0))
    (else
      (set `self.KnobRotate` (struct))
      (set `self.OffsetKnob` _returnvalue_3)))
  (`SceneComponent.K2_SetRelativeLocationAndRotation` (`self.SM_Knob`) (`KismetMathLibrary.MakeVector` 0.0 (`self.OffsetKnob`) 100.0) (`self.KnobRotate`) false true)
  (`SceneComponent.K2_SetRelativeLocation` (`self.SM_HingesBottom`) (`KismetMathLibrary.MakeVector` -0.5 (`self.OffsetScene`) 27.0) false true)
  (`SceneComponent.K2_SetRelativeLocation` (`self.SM_HingesTop`) (`KismetMathLibrary.MakeVector` -0.5 (`self.OffsetScene`) 170.0) false true)
  (`SceneComponent.K2_SetRelativeLocation` (`self.Target`) (`KismetMathLibrary.MakeVector` 0.0 (`self.OffsetKnob`) 100.0) false true)
  ;[1 1 1] If door opened then return rotate of scene to Opened rotation
  (if (`self.DoorOpenStatus`)
    (`SceneComponent.K2_SetRelativeRotation` (`self.Scene`) (`self.EndDoor`) false true))
  (return))

(fn `UserConstructionScript`
  (bind _smarray (`self.SMArray`))
  (bind _staticmeshcomponent (`self.StaticMeshComponent`))
  (`StaticMeshComponent.SetStaticMesh` _staticmeshcomponent (`self.DoorHinges`))
  (`SceneComponent.SetHiddenInGame` _staticmeshcomponent true false)
  (`StaticMeshComponent.SetStaticMesh` (`self.SM_Frame`) (`self.Frame`))
  (`StaticMeshComponent.SetStaticMesh` (`self.SM_TrimInSide`) (`self.TrimInSide`))
  (`StaticMeshComponent.SetStaticMesh` (`self.SM_TrimOutSide`) (`self.TrimOutSide`))
  (`StaticMeshComponent.SetStaticMesh` (`self.SM_Door`) (`self.Door`))
  (`StaticMeshComponent.SetStaticMesh` (`self.SM_HingesTop`) (`self.DoorHinges`))
  (`StaticMeshComponent.SetStaticMesh` (`self.SM_HingesBottom`) (`self.DoorHinges`))
  (`StaticMeshComponent.SetStaticMesh` (`self.SM_Knob`) (`self.Knob`))
  (set `self.Width` (.y (`.Max` (`StaticMeshComponent.GetLocalBounds` (`self.SM_Door`)))))
  (`self.SetupDoor`)
  (`KismetArrayLibrary.Array_Clear` _smarray)
  (`KismetArrayLibrary.Array_Add` _smarray (`self.SM_Door`))
  (for _array_element (`self.SMArray`)
    (`PrimitiveComponent.SetRenderCustomDepth` _array_element false)
    (`PrimitiveComponent.SetCustomDepthStencilValue` _array_element (`self.DepthStencilValue`))
    (`PrimitiveComponent.SetSimulatePhysics` _array_element false)))