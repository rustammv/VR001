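; BP_Measure is an actor that visualizes the distance between two points with end markers, a connecting line and a text label.
; SetFirstPoint places the first marker and creates a spline mesh.
; SetSecondPoint stretches it between the markers, inset by marker size, and shows the rounded distance at the midpoint, facing the camera's yaw.
; OnDestroyMeasure starts a retriggerable delay before destruction, during which Tick keeps turning the label toward the camera.
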(event `/Game/Interface/I_Measure.OnDestroyMeasure`
  ;[0.2135 0.2135 0.2135 1 12] OnDestroyMeasure удаляем эктора через время Times
  (set `self.IsDestroy` true)
  (`KismetSystemLibrary.RetriggerableDelay` (`self.Timer`))
  (`self.K2_DestroyActor`))

(event `/Game/Interface/I_Measure.SetFirstPoint`
  (params (Pos :type "Vector Structure"))
  ;[1 1 1] Comment
  (bind _output_get (set `self.PosFirst` Pos))
  (`SceneComponent.K2_SetWorldLocationAndRotation` :`self` (`self.First`) :`NewLocation` _output_get :`bTeleport` true)
  (bind _returnvalue (`AddComponent|NODE_AddSplineMeshComponent-1` :`bManualAttachment` true))
  (set `self.splineMesh` _returnvalue)
  ;;[0.2135 0.2135 0.2135 1 12] устанавливаем тип точек сплайна
  (`SplineComponent.SetSplinePointType` (`self.Spline`) 0 "Constant" true)
  (`SplineComponent.SetSplinePointType` (`self.Spline`) 1 "Constant" true)
  ;;[0.2135 0.2135 0.2135 1 12] вычисляем смещение линии от точек в зависимости от размера Point мешей
  (set `self.Offset` (* (.z (`.BoxExtent` (`KismetSystemLibrary.GetComponentBounds` (`self.PointFirst`)))) 2.0)))

(event `/Game/Interface/I_Measure.SetSecondPoint`
  (params (Pos :type "Vector Structure"))
  (bind (_returnvalue_roll _returnvalue_pitch _returnvalue_yaw) (`KismetMathLibrary.BreakRotator` (`SceneComponent.K2_GetComponentRotation` (`PlayerCameraManager.TransformComponent` (`GameplayStatics.GetPlayerCameraManager` 0)))))
  (bind _output_get (set `self.PosSecond` Pos))
  (`SceneComponent.K2_SetWorldLocationAndRotation` :`self` (`self.Second`) :`NewLocation` _output_get :`bTeleport` true)
  ;[0.2135 0.2135 0.2135 1 12] Получаем растояние между точками
  (set `self.Distance` (`KismetMathLibrary.VSize` (- (`self.PosSecond`) (`self.PosFirst`))))
  ;[0.2135 0.2135 0.2135 1 12] рисуем линию между точками
  (`SplineMeshComponent.SetStartAndEnd` (`self.splineMesh`) (+ (`self.PosFirst`) (* (`KismetMathLibrary.GetDirectionUnitVector` (`self.PosFirst`) (`self.PosSecond`)) (`self.Offset`))) (0.0 0.0 0.0) (+ (`self.PosSecond`) (* (`KismetMathLibrary.GetDirectionUnitVector` (`self.PosSecond`) (`self.PosFirst`)) (`self.Offset`))) (0.0 0.0 0.0) true)
  (`SplineMeshComponent.SetEndScale` (`self.splineMesh`) (`self.BeamScale`) true)
  (`SplineMeshComponent.SetStartScale` (`self.splineMesh`) (`self.BeamScale`) true)
  ;[0.2083 0.2083 0.2083 1 12] Получем координаты середины между точками
  (bind _output_get_2 (set `self.PosText` (+ (`self.PosSecond`) (* (`KismetMathLibrary.GetDirectionUnitVector` (`self.PosSecond`) (`self.PosFirst`)) (/ (`self.Distance`) 2.0)))))
  ;[0.2135 0.2135 0.2135 1 12] поворачиваем текст в камеру
  (`SceneComponent.K2_SetWorldLocationAndRotation` (`self.Text`) _output_get_2 (`KismetMathLibrary.MakeRotator` 0.0 0.0 (+ _returnvalue_yaw 180.0)) false true)
  ;[0.2135 0.2135 0.2135 1 12] записываем округлённую дистанцию в секстовое поле
  (set `self.TextMeasure` (`KismetTextLibrary.Conv_IntToText` (`KismetMathLibrary.Round` (`self.Distance`)) false true 1 10))
  (`TextRenderComponent.K2_SetText` (`self.TextRender`) (`self.TextMeasure`)))

(event `self.ReceiveBeginPlay`
  (bind _scalepoint (`self.ScalePoint`))
  (bind _scalepoint_2 (`self.ScalePoint`))
  ;[0.2135 0.2135 0.2135 1 12] устанавливаем Scale для Point мешей
  (`SceneComponent.SetRelativeScale3D` (`self.First`) (`KismetMathLibrary.MakeVector` _scalepoint _scalepoint _scalepoint))
  (`SceneComponent.SetRelativeScale3D` (`self.Second`) (`KismetMathLibrary.MakeVector` _scalepoint_2 _scalepoint_2 _scalepoint_2)))

(event `self.ReceiveTick`
  (params (DeltaSeconds :type "Float (single-precision)"))
  (bind (_returnvalue_roll _returnvalue_pitch _returnvalue_yaw) (`KismetMathLibrary.BreakRotator` (`SceneComponent.K2_GetComponentRotation` (`PlayerCameraManager.TransformComponent` (`GameplayStatics.GetPlayerCameraManager` 0)))))
  (if (`self.IsDestroy`)
    (`SceneComponent.K2_SetWorldRotation` (`self.Text`) (`KismetMathLibrary.MakeRotator` 0.0 0.0 (+ _returnvalue_yaw 180.0)) false true)))

(fn `UserConstructionScript`)