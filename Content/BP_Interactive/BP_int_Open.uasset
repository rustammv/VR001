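; Interactive prop assembled from a data array of mesh parts, each hung on its own pivot for opening.
; Construction script builds each part's pivot, offset mesh and hidden debug cube, adding a knob trigger sphere to openable parts.
; It sets each part's highlight stencil value with custom depth off.
; Tick constantly spins the second part's pivot by a fixed per-frame step; no overlap or open logic is implemented.
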(event `self.ReceiveActorBeginOverlap`
  (params (OtherActor :type "Actor Object Reference")))

(event `self.ReceiveTick`
  (params (DeltaSeconds :type "Float (single-precision)"))
  (bind (_output_mesh _output_meshcomponent _output_scene) (break `/Game/Struct/Struct_Fridge` (`|GetArrayItem` (`self.Meshes`) 1)))
  (`parent.ReceiveTick` DeltaSeconds)
  (`SceneComponent.K2_AddRelativeRotation` _output_scene (struct :`Yaw` 1.0) false true))

(fn `UpdateArray`
  (params (IN :type "/Game/Struct/Struct_Fridge Structure") (Index :type Integer))
  (returns (Out :type "/Game/Struct/Struct_Fridge Structure"))
  (locals (temp :type "/Game/Struct/Struct_Fridge Structure"))
  (`|ExecutionSequence`
    (:`then_0`
      (`/Engine/EditorBlueprintResources/StandardMacros.IsValid` IN_Mesh_5_33F09FE2491BC27A38B673A54FF8AAC1
        (:`Is Valid`
          (bind _output_get (set `local.temp` (make `/Game/Struct/Struct_Fridge` IN_Mesh_5_33F09FE2491BC27A38B673A54FF8AAC1)))
          (`KismetArrayLibrary.Array_Set` (`self.Meshes`) Index (make `/Game/Struct/Struct_Fridge` (break `/Game/Struct/Struct_Fridge` _output_get)))
          (return (make `/Game/Struct/Struct_Fridge` null)))))))

(fn `UserConstructionScript`
  (locals (Index :type Integer) (RadiusCollisionKnob :type "Float (double-precision)" :default 15.0))
  (bind (_output_mesh _output_meshcomponent _output_scene _output_pivot) (break `/Game/Struct/Struct_Fridge` (`|GetArrayItem` (`self.Meshes`) (`local.Index`))))
  (bind _output (`|GetArrayItem` (`self.Meshes`) (`local.Index`)))
  (bind (_output_mesh_2 _output_meshcomponent_2 _output_scene_2 _output_pivot_2 _output_offsetmesh _output_rotatemesh _output_openable _output_offsettrigger) (break `/Game/Struct/Struct_Fridge` (`|GetArrayItem` (`self.Meshes`) (`local.Index`))))
  (bind (_output_mesh_3 _output_meshcomponent_3 _output_scene_3 _output_pivot_3) (break `/Game/Struct/Struct_Fridge` (`|GetArrayItem` (`self.Meshes`) (`local.Index`))))
  (bind (_output_mesh_4 _output_meshcomponent_4) (break `/Game/Struct/Struct_Fridge` (`|GetArrayItem` (`self.Meshes`) (`local.Index`))))
  (bind (_output_mesh_5 _output_meshcomponent_5 _output_scene_4 _output_pivot_4) (break `/Game/Struct/Struct_Fridge` (`|GetArrayItem` (`self.Meshes`) (`local.Index`))))
  (bind (_output_mesh_6 _output_meshcomponent_6 _output_scene_5 _output_pivot_5 _output_offsetmesh_2 _output_rotatemesh_2) (break `/Game/Struct/Struct_Fridge` (`|GetArrayItem` (`self.Meshes`) (`local.Index`))))
  (bind (_output_mesh_7 _output_meshcomponent_7 _output_scene_6 _output_pivot_6 _output_offsetmesh_3 _output_rotatemesh_3 _output_openable_2 _output_offsettrigger_2 _output_highlightable _output_description) (break `/Game/Struct/Struct_Fridge` (`|GetArrayItem` (`self.Meshes`) (`local.Index`))))
  (`parent.UserConstructionScript`)
  (bind _returnvalue (`AddComponent|NODE_AddSceneComponent-2` :`bManualAttachment` true))
  (bind _output_get (set `self.SceneRoot` _returnvalue))
  (`SceneComponent.K2_AttachToComponent` _output_get (`self.StaticMeshComponent`) "None" "KeepRelative" "KeepRelative" "KeepRelative" false)
  (for (_ _array_index) (`self.Meshes`)
    (set `local.Index` _array_index)
    (bind _returnvalue_2 (`AddComponent|NODE_AddSceneComponent-1` :`bManualAttachment` true :`RelativeTransform` (`KismetMathLibrary.MakeTransform` _output_pivot_4)))
    (`SceneComponent.K2_AttachToComponent` _returnvalue_2 (`self.SceneRoot`) "None" "KeepRelative" "KeepRelative" "KeepRelative" false)
    (`SceneComponent.K2_SetRelativeLocation` (`self.StaticMesh`) _output_pivot_3 false true)
    (bind _returnvalue_3 (`AddComponent|NODE_AddStaticMeshComponent-1` :`bManualAttachment` true :`RelativeTransform` (`KismetMathLibrary.MakeTransform` _output_pivot (struct) (0.1 0.1 0.1))))
    (`StaticMeshComponent.SetStaticMesh` _returnvalue_3 "/Game/Meshes/1M_Cube.1M_Cube")
    (`SceneComponent.SetHiddenInGame` _returnvalue_3 true false)
    (`SceneComponent.K2_AttachToComponent` _returnvalue_3 _returnvalue_2 "None" "SnapToTarget" "SnapToTarget" "KeepRelative" true)
    (bind _returnvalue_4 (`AddComponent|NODE_AddStaticMeshComponent-0` :`bManualAttachment` true))
    (`SceneComponent.K2_AttachToComponent` _returnvalue_4 _returnvalue_2 "None" "KeepRelative" "KeepRelative" "KeepRelative" false)
    (`KismetArrayLibrary.Array_Set` (`self.Meshes`) (`local.Index`) (make `/Game/Struct/Struct_Fridge` _output_mesh_7 _returnvalue_4 _returnvalue_2 _output_pivot_6 _output_offsetmesh_3 _output_rotatemesh_3 _output_openable_2 _output_offsettrigger_2 _output_highlightable _output_description))
    (`SceneComponent.K2_SetRelativeLocationAndRotation` _output_meshcomponent_6 _output_offsetmesh_2 _output_rotatemesh_2 false true)
    (`StaticMeshComponent.SetStaticMesh` _output_meshcomponent_4 _output_mesh_4)
    (`|ExecutionSequence`
      (:`then_0`
        (if _output_openable
          (bind _returnvalue_5 (`AddComponent|NODE_AddSphereComponent-0` :`bManualAttachment` true :`RelativeTransform` (`KismetMathLibrary.MakeTransform` _output_offsettrigger)))
          (`SphereComponent.SetSphereRadius` _returnvalue_5 (`local.RadiusCollisionKnob`) true)
          (`SceneComponent.K2_AttachToComponent` _returnvalue_5 _output_meshcomponent_2 "None" "KeepRelative" "KeepRelative" "KeepRelative" false)))
      (:`then_1`
        (`PrimitiveComponent.SetRenderCustomDepth` (`.MeshComponent_29_C31FBD9948BC7A497EE95E9E1F9D364B` (break `/Game/Struct/Struct_Fridge` _output)) false)
        (`PrimitiveComponent.SetCustomDepthStencilValue` (`.MeshComponent_29_C31FBD9948BC7A497EE95E9E1F9D364B` (break `/Game/Struct/Struct_Fridge` _output)) (`.DepthStencil_4_8B3AFAF242DA3141F48409A63BC45252` (break `/Game/Struct/Struct_HighLightable` (`.HighLightable_20_58BC955B4A0C8318BB2E3AAF98456483` (break `/Game/Struct/Struct_Fridge` _output)))))))))