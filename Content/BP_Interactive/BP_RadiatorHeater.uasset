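; BP_RadiatorHeater is a procedural radiator heater prop assembled from static mesh components.
; The Construction Script adds two vertically stacked valve meshes, then repeats a section mesh along Y for the configured section count, all shifted by pivot offsets.
; The valve connection side, left or right, flips the valves' roll and the direction the sections extend.
; The event graph holds only disabled stub events, so it has no runtime logic.
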(fn `UserConstructionScript`
  (locals (indexSections :type Integer) (WightSection :type "Float (double-precision)" :default 8.0) (indexValve :type Integer) (SideCorrection :type "Float (double-precision)") (AngleCorrection :type "Float (double-precision)" :default 90.0))
  (bind _output (`|GetArrayItem` (`self.SMComponents`) (`local.indexValve`)))
  (bind _output_2 (`|GetArrayItem` (`self.SMComponents`) (+ (`local.indexSections`) 1)))
  (switch `/Game/Enum/Enum_Side` (`self.ValveConnectionSide`)
    (:`NewEnumerator0`
      (set `local.SideCorrection` 1.0)
      (set `local.AngleCorrection` 180.0))
    (:`NewEnumerator1`
      (set `local.SideCorrection` -1.0)
      (set `local.AngleCorrection` 0.0)))
  (`StaticMeshComponent.SetStaticMesh` (`self.StaticMeshComponent`) null)
  (for _index (range 2)
    (set `local.indexValve` _index)
    (bind _returnvalue (`AddComponent|NODE_AddStaticMeshComponent-1`))
    (`KismetArrayLibrary.Array_Add` (`self.SMComponents`) _returnvalue)
    (`StaticMeshComponent.SetStaticMesh` _output (`self.Valve`))
    (`SceneComponent.K2_SetRelativeLocationAndRotation` _output (`KismetMathLibrary.MakeVector` (`self.OffSetPivotX`) (+ (* (`local.indexSections`) (`local.WightSection`)) (* (`local.SideCorrection`) 3.05) (`self.OffSetPivotY`)) (+ (* (`local.indexValve`) -50.0) (`self.OffSetPivotZ`))) (`KismetMathLibrary.MakeRotator` (`local.AngleCorrection`)) false false))
  ;[1 1 1] Create need amount of section
  (for _index_2 (range 1 (+ (- (`self.AmountSections`) 0) 1))
    (set `local.indexSections` _index_2)
    (bind _returnvalue_2 (`AddComponent|NODE_AddStaticMeshComponent-0`))
    (`KismetArrayLibrary.Array_Add` (`self.SMComponents`) _returnvalue_2)
    (`StaticMeshComponent.SetStaticMesh` _output_2 (`self.RadiatorPart`))
    (`SceneComponent.K2_SetRelativeLocation` _output_2 (`KismetMathLibrary.MakeVector` (`self.OffSetPivotX`) (+ (* (* (+ (`local.indexSections`) 0) (`local.WightSection`)) (`local.SideCorrection`)) (* (`local.SideCorrection`) -1.0) (`self.OffSetPivotY`)) (`self.OffSetPivotZ`)) false true)))