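; BP_Roller is a configurable roller prop, apparently a window blind, with rolls, side picks, a hanging plane and a wire.
; The construction script scales and positions the meshes from Width and Height, with extra wire length and a selectable wire side.
; It applies one material to the plane and a shared plastic material to the other parts.
; The event graph holds only disabled stubs, so it has no runtime logic.
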(event EventBeginPlay)

(event Collision|EventActorBeginOverlap
  (params (OtherActor :type Actor%20Object%20Reference)))

(event EventTick
  (params (DeltaSeconds :type Float%20%28single-precision%29)))

(fn ConstructionScript
  (Variables|Default|SetScaleWidth (|(1/(100/{2C2C6A85-4453-A8DF-C358-E1B29FF0AE12}))))
  (Variables|Default|SetOffSetWidthPick (+ (/ (Variables|Default|GetWidth) 2.0) 1.5))
  (Variables|Default|SetScaleHeight (|({B2EE7BB3-46A9-7F95-BB5E-68BA794432ED}/100)))
  (Variables|Default|SetScaleHeightWire (|(({B2EE7BB3-46A9-7F95-BB5E-68BA794432ED}+{17724795-44BA-752D-BEAE-1EBFBA93BAF2})/100)))
  (Transformation|SetRelativeTransform (Variables|Default|GetSM_RollUp) (Math|Transform|MakeTransform "0, 0, 0" "0, 0, 0" (Math|Vector|MakeVector (Variables|Default|GetScaleWidth) 1.0 1.0)) false false)
  (Transformation|SetRelativeTransform (Variables|Default|GetSM_RollDown) (Math|Transform|MakeTransform (Math|Vector|MakeVector 0.0 0.0 (* (Variables|Default|GetHeight) -1.0)) "0, 0, 0" (Math|Vector|MakeVector (Variables|Default|GetScaleWidth) 1.0 1.0)) false false)
  (Transformation|SetRelativeLocation (Variables|Default|GetSM_PickLeft) (Math|Vector|MakeVector (Variables|Default|GetOffSetWidthPick) 0.0 0.0) false true)
  (Transformation|SetRelativeLocation (Variables|Default|GetSM_PickRight) (Math|Vector|MakeVector (* (Variables|Default|GetOffSetWidthPick) -1.0) 0.0 0.0) false true)
  (Transformation|SetRelativeTransform (Variables|Default|GetSM_Plane) (Math|Transform|MakeTransform "0,2.200000, 0" "0, 0, 0" (Math|Vector|MakeVector (Variables|Default|GetScaleWidth) 1.0 (Variables|Default|GetScaleHeight))) false false)
  (if (Variables|Default|GetSideWire)
    (Variables|Default|SetOffSetWidthWire (* (+ (Variables|Default|GetOffSetWidthPick) -1.0) -1.0))
    (else
      (Variables|Default|SetOffSetWidthWire (+ (Variables|Default|GetOffSetWidthPick) -1.0))))
  (Transformation|SetRelativeTransform (Variables|Default|GetSM_Wire) (Math|Transform|MakeTransform (Math|Vector|MakeVector (Variables|Default|GetOffSetWidthWire) 3.0 0.0) "0, 0, 0" (Math|Vector|MakeVector 1.0 1.0 (Variables|Default|GetScaleHeightWire))) false false)
  (Rendering|Material|SetMaterial (Variables|Default|GetSM_Plane) 0 (Variables|Default|GetMaterialPlane))
  (Rendering|Material|SetMaterial (Variables|Default|GetSM_RollUp) 0 (Variables|Default|GetMaterialPlastic))
  (Rendering|Material|SetMaterial (Variables|Default|GetSM_RollDown) 0 (Variables|Default|GetMaterialPlastic))
  (Rendering|Material|SetMaterial (Variables|Default|GetSM_PickLeft) 0 (Variables|Default|GetMaterialPlastic))
  (Rendering|Material|SetMaterial (Variables|Default|GetSM_PickRight) 0 (Variables|Default|GetMaterialPlastic))
  (Rendering|Material|SetMaterial (Variables|Default|GetSM_Wire) 0 (Variables|Default|GetMaterialPlastic)))